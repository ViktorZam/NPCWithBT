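; AC_Allies is an actor component that sets up its owning character as an AI ally.
; On BeginPlay it sets the owner's capsule collision object type to Pawn, then has the owner's AI controller run the BT_Allies behavior tree.
; Getter functions identify the component: GetAlliesAC returns itself, while GetSummonerAC returns nothing.
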(event EventBeginPlay
  (|CallParentFunction)
  (Collision|SetCollisionObjectType (Variables|/Script/Engine.Character|GetCapsuleComponent (Variables|Default|GetOwner)) "ECC_Pawn")
  (AI|RunBehaviorTree (AI|GetAIController (Variables|Default|GetOwner)) "/Game/Blueprints/AI/BT/BT/BT_Allies.BT_Allies"))

(fn GetAlliesAC
  (return self))

(fn GetSummonerAC
  (return 0))