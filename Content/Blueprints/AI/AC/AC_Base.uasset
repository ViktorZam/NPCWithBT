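; AC_Base is a base Actor Component that lets characters capture each other, converting targets to the player's or AI's side.
; Capture swaps tagged components for AC_Allies or AC_Summoner, stops movement and montages, and updates the GameMode's possessed-character list and HUD score.
; A captured player hands control to the first possessed character, or the game quits if none remain.
; The component getters are empty stubs.
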(event EventBeginPlay
  (bind _thirdpersoncharacter (Class|BPIAI|GetThirdPersonCharacter(Message) (Components|GetOwner)))
  (Variables|Default|SetOwner _thirdpersoncharacter))

(fn CaptureAnotherAI
  (params (TagConquare :type Name) (TargetCapture :type BP%20Third%20Person%20Character%20Object%20Reference))
  (LocalVariables|SetL_TargetCapture TargetCapture)
  (switch name TagConquare
    (:Player
      (CallFunction|HandleCaptureAI (LocalVariables|GetL_TargetCapture) "AI" true "/Game/Blueprints/AI/AC/AC_Allies.AC_Allies_C"))
    (:AI
      (if (== (LocalVariables|GetL_TargetCapture) (Game|GetPlayerCharacter 0))
        (CallFunction|HandleCaptureAI (LocalVariables|GetL_TargetCapture) "Player" false "/Game/Blueprints/AI/AC/AC_Summoner.AC_Summoner_C")
        (else
          (CallFunction|HandleCaptureAI (LocalVariables|GetL_TargetCapture) "AI" false "/Game/Blueprints/AI/AC/AC_Summoner.AC_Summoner_C"))))))

(fn HandleCaptureAI
  (params (TargetCapture :type BP%20Third%20Person%20Character%20Object%20Reference) (TagDestroyedComponent :type Name) (IncAlly? :type Boolean) (ConquareClass :type Actor%20Component%20Class%20Reference))
  (Default|DestroyOwnComponents TargetCapture TagDestroyedComponent)
  (bind _gm (Class|BPIGM|GetGMThirdPerson(Message) (Game|GetGameMode)))
  (LocalVariables|SetL_GM _gm)
  (Class|NavMovementComponent|StopActiveMovement (Variables|/Script/Engine.Character|GetCharacterMovement TargetCapture))
  (Animation|StopAnimMontage TargetCapture (Animation|GetCurrentMontage TargetCapture :!class /Script/Engine.Character))
  (Default|IncDecPosessesCharacters (LocalVariables|GetL_GM) TargetCapture IncAlly?)
  (if (!= TagDestroyedComponent "Player")
    (Game|AddComponentbyClass TargetCapture ConquareClass :!label _label)
    (bind _hud (Class|BPIHUD|GetHUD(Message) (HUD|GetHUD (Game|GetPlayerController 0))))
    (Default|ChangeScore (Variables|/Game/Blueprints/BP_HUD.BP_HUD_C|GetInfoWidget _hud) IncAlly?)
    (elif (!= (Utilities|Array|Length (Variables|/Game/Blueprints/BP_ThirdPersonGameMode.BP_ThirdPersonGameMode_C|GetPosessesCharacters (LocalVariables|GetL_GM))) 0)
      (Default|PosessesAfterEnemyCapturedPlayer (Utilities|Array|Get(acopy) (Variables|/Game/Blueprints/BP_ThirdPersonGameMode.BP_ThirdPersonGameMode_C|GetPosessesCharacters (LocalVariables|GetL_GM))))
      (Default|CheckSelfAIController TargetCapture)
      (goto _label)
      (else
        (Game|QuitGame 0 "Quit" false)))))

(fn GetAlliesAC
  (return 0))

(fn GetPlayerAC
  (return 0))

(fn GetSummonerAC
  (return 0))