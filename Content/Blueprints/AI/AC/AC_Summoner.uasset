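; Actor component that turns its owner into an AI summoner NPC.
; On BeginPlay it adds tagged summon-point scene components and a hidden screen-space WBP_Q widget, changes the capsule's collision channel, runs BT_Summoner and saves the start location to the blackboard.
; On EndPlay it destroys the actors in Zombies and removes the tagged components.
; The summoning itself is not in this graph; GetSummonerAC exposes the component.
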(event EventBeginPlay
  (|CallParentFunction)
  (CallFunction|CreatePointsOfSpawn)
  (CallFunction|CreateWidgetQ)
  (Collision|SetCollisionObjectType (Variables|/Script/Engine.Character|GetCapsuleComponent (Variables|Default|GetOwner)) "ECC_GameTraceChannel2")
  (AI|RunBehaviorTree (AI|GetAIController (Variables|Default|GetOwner)) "/Game/Blueprints/AI/BT/BT/BT_Summoner.BT_Summoner")
  (AI|Components|Blackboard|SetValueasVector (AI|GetBlackboard (Variables|Default|GetOwner)) (Utilities|Name|MakeLiteralName "StartPointLocationNPC") (Transformation|GetActorLocation (Variables|Default|GetOwner))))

(event EventEndPlay
  (params (EndPlayReason :type EEndPlayReason%20Enum :default "Destroyed"))
  (|CallParentFunction EndPlayReason)
  (for _array_element (Variables|Default|GetZombies)
    (Actor|DestroyActor _array_element))
  (Default|DestroyOwnComponents (Variables|Default|GetOwner) "PointOfSummon")
  (Default|DestroyOwnComponents (Variables|Default|GetOwner) "Widget"))

(fn GetSummonerAC
  (return self))

(fn CreatePointsOfSpawn
  (for _array_element (Utilities|Array|MakeArray "130.000000,210.000000,0.000000" "200.000000,100.000000,0.000000" "30.000000,-140.000000,0.000000" "-180.000000,-60.000000,0.000000")
    (bind _returnvalue (Game|AddComponentbyClass (Variables|Default|GetOwner) "/Script/Engine.SceneComponent" false (Math|Transform|MakeTransform _array_element "0, 0, 0" "1.000000,1.000000,1.000000"))) ; 1
    (Utilities|Array|Add (Variables|/Script/Engine.ActorComponent|GetComponentTags _returnvalue) "PointOfSummon")))

(fn CreateWidgetQ
  (bind _returnvalue (Game|AddComponentbyClass (Variables|Default|GetOwner) "/Script/UMG.WidgetComponent" false (Math|Transform|MakeTransform "0.000000,0.000000,110.000000" "0, 0, 0" "1.000000,1.000000,1.000000")))
  (bind _output_get (Variables|Default|SetQWidget _returnvalue))
  (Utilities|Array|Add (Variables|/Script/Engine.ActorComponent|GetComponentTags _output_get) "Widget")
  (bind _returnvalue_2 (UserInterface|CreateWidget "/Game/UI/Widgets/WBP_Q.WBP_Q_C"))
  (UserInterface|SetWidget (Variables|Default|GetQWidget) _returnvalue_2)
  (Class|WidgetComponent|SetDrawatDesiredSize (Variables|Default|GetQWidget) true)
  (Collision|SetCollisionEnabled (Variables|Default|GetQWidget) "NoCollision")
  (Class|WidgetComponent|SetWidgetSpace (Variables|Default|GetQWidget) "Screen")
  (Development|SetHiddeninGame (Variables|Default|GetQWidget) true false))