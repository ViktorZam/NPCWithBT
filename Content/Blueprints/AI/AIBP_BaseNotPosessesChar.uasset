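; Base Blueprint for an AI-driven, non-possessed character that runs the BT_Summoner behavior tree.
; On BeginPlay it starts the tree on its AI controller, then stores its spawn location in the StartPointLocationNPC blackboard key.
; GetThirdPersonCharacter and GetZombie are empty stubs, and the construction script does nothing.
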(event EventBeginPlay
  (AI|RunBehaviorTree (AI|GetAIController self) "/Game/Blueprints/AI/BT/BT/BT_Summoner.BT_Summoner")
  (AI|Components|Blackboard|SetValueasVector (AI|GetBlackboard 0) (Utilities|Name|MakeLiteralName "StartPointLocationNPC") (Transformation|GetActorLocation)))

(fn ConstructionScript)

(fn GetThirdPersonCharacter
  (return 0))

(fn GetZombie
  (return 0))