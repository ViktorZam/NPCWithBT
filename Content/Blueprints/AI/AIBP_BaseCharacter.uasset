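; Base AI character Blueprint that starts NPC behavior when play begins.
; On BeginPlay its AI controller runs BT_BaseCharacter, then the character's current location is written to the blackboard key StartPointLocationNPC as its start point.
; GetSummonerCharacter and GetZombie are empty stubs that return no values here, and the construction script is empty.
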(event EventBeginPlay
  (AI|RunBehaviorTree (AI|GetAIController self) "/Game/Blueprints/AI/BT_BaseCharacter.BT_BaseCharacter")
  (AI|Components|Blackboard|SetValueasVector (AI|GetBlackboard 0) (Utilities|Name|MakeLiteralName "StartPointLocationNPC") (Transformation|GetActorLocation)))

(fn ConstructionScript)

(fn GetSummonerCharacter
  (return 0))

(fn GetZombie
  (return 0))