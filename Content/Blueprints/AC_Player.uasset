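; Player actor component that detects a summoner enemy in front of the owner and toggles its QWidget prompt.
; A looping timer set at BeginPlay appears to drive CheckSummoner, which box-traces ahead and filters hits by relative yaw.
; It tracks one EnemyTarget, reaching the widget through that actor's "AI"-tagged component.
; The widget hides when the target is lost, replaced or play ends.
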(event EventBeginPlay
  (|CallParentFunction)
  (Collision|SetCollisionObjectType (Variables|/Script/Engine.Character|GetCapsuleComponent (Variables|Default|GetOwner)) "ECC_Pawn")
  (Utilities|Time|SetTimerbyEvent (EventDispatchers|CreateEvent :!event CheckSummoner) 0.3 true))

(event EventEndPlay
  (params (EndPlayReason :type EEndPlayReason%20Enum :default "Destroyed"))
  (|CallParentFunction EndPlayReason)
  (Utilities|IsValid (Variables|Default|GetEnemyTarget)
    (:Is%20Valid
      (CallFunction|HideWidget true)
      (Variables|Default|SetEnemyTarget 0))))

(fn HideWidget
  (params (Hide? :type Boolean))
  (bind _acsummoner (Class|BPIAC|GetSummonerAC(Message) (Utilities|Array|Get(acopy) (Actor|GetComponentsbyTag (Variables|Default|GetEnemyTarget) "/Script/Engine.ActorComponent" "AI"))))
  (Utilities|IsValid _acsummoner
    (:Is%20Valid
      (Development|SetHiddeninGame (Variables|/Game/Blueprints/AI/AC/AC_Summoner.AC_Summoner_C|GetQWidget _acsummoner) Hide? false))))

(fn CheckSummoner
  (bind _owner (Variables|Default|GetOwner))
  (bind _owner_2 (Variables|Default|GetOwner))
  (bind _returnvalue (Transformation|GetActorLocation _owner_2))
  (bind _returnvalue_2 (Transformation|GetActorForwardVector _owner))
  (bind _returnvalue_3 (* _returnvalue_2 1e+02))
  (bind _returnvalue_4 (+ _returnvalue_3 _returnvalue))
  (bind (_outhit _returnvalue_5) (Class|KismetSystemLibrary|BoxTraceSingleforObjects _returnvalue_4 _returnvalue_4 "100.000000,100.000000,50.000000" (Math|Rotator|MakeRotator 0.0 0.0 (.yaw (Transformation|GetActorRotation (Variables|Default|GetOwner)))) (Utilities|Array|MakeArray "ObjectTypeQuery7") false 0 "ForDuration" true))
  (if _returnvalue_5
    (LocalVariables|SetL_HitActor (.HitActor (Collision|BreakHitResult _outhit)))
    (if (> (.yaw (Math|Rotator|Delta(Rotator) (Transformation|GetActorRotation (LocalVariables|GetL_HitActor)) (Transformation|GetActorRotation (Variables|Default|GetOwner)))) 7e+01)
      (Utilities|IsValid (Variables|Default|GetEnemyTarget)
        (:Is%20Valid
          (if (> (Transformation|GetDistanceTo (Variables|Default|GetEnemyTarget) (Variables|Default|GetOwner)) 1e+02)
            (CallFunction|HideWidget true)
            (Variables|Default|SetEnemyTarget 0)
            (elif (> (.yaw (Math|Rotator|Delta(Rotator) (Transformation|GetActorRotation (Variables|Default|GetEnemyTarget)) (Transformation|GetActorRotation (Variables|Default|GetOwner)))) 7e+01)
              (CallFunction|HideWidget true)
              (Variables|Default|SetEnemyTarget 0)))))
      (elif (== (Variables|Default|GetEnemyTarget) (LocalVariables|GetL_HitActor))
        (CallFunction|HideWidget false)
        (else
          (Utilities|IsValid (Variables|Default|GetEnemyTarget)
            (:Is%20Valid
              (CallFunction|HideWidget true))
            (:Is%20Not%20Valid
              _))
          (Variables|Default|SetEnemyTarget (LocalVariables|GetL_HitActor))
          (CallFunction|HideWidget false))))
    (else
      (Utilities|IsValid (Variables|Default|GetEnemyTarget)
        (:Is%20Valid
          (CallFunction|HideWidget true)
          (Variables|Default|SetEnemyTarget 0))))))

(fn GetPlayerAC
  (return self))